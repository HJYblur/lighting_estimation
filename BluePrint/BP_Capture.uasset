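; BP_Capture is a key-driven capture tool that produces numbered screenshots under randomized directional lighting.
; Pressing C randomizes the light's intensity and temperature and requests a high-res portrait screenshot; releasing C increments the index.
; Each capture prints its lighting labels, including light rotation in follow-camera space, intensity, color, temperature and image name.
; Camera-rotation and light-color randomization are present but disconnected, so they never run.
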(event `Count Time`
  (bind _output_get (set `self.Cnt` (+ (`self.Cnt`) 1)))
  (if (== _output_get 100)
    (set `self.Cnt` 0)))

(event `self.ReceiveBeginPlay`
  (bind _asbp_third_person_character (cast `/Game/ThirdPerson/Blueprints/BP_ThirdPersonCharacter` (`GameplayStatics.GetPlayerPawn` 0)))
  (set `self.CurrentRotation` (`SceneComponent.K2_GetComponentRotation` (`/Game/ThirdPerson/Blueprints/BP_ThirdPersonCharacter.FollowCamera` _asbp_third_person_character))))

(event `self.ReceiveTick`
  (params (DeltaSeconds :type "Float (single-precision)")))

(event `Key|C`
  (params (Key :type "Key Structure"))
  (bind _lightcomponent (`Light.LightComponent` (`self.DirectionalLight`)))
  (bind _lightcomponent_2 (`Light.LightComponent` (`self.DirectionalLight`)))
  (:`Pressed`
    (`|ExecutionSequence`
      (:`then_0`
        (`LightComponent.SetIntensity` _lightcomponent (`KismetMathLibrary.RandomFloatInRange` 100000.0 500000.0))
        (`LightComponent.SetTemperature` _lightcomponent (`KismetMathLibrary.RandomFloatInRange` 2500.0 6500.0))
        (`AbilitySystemBlueprintLibrary.SetDuration` (struct) 0.3))
      (:`then_2`
        (`AutomationBlueprintFunctionLibrary.TakeHighResScreenshot` 1280 1920 (`KismetStringLibrary.Concat_StrStr` (`self.screenshot`) (`KismetStringLibrary.Conv_IntToString` (`self.num`)) ".png") null)
        (bind _asbp_third_person_character (cast `/Game/ThirdPerson/Blueprints/BP_ThirdPersonCharacter` (`GameplayStatics.GetPlayerPawn` 0)))
        (`KismetSystemLibrary.PrintString` (`KismetStringLibrary.Concat_StrStr` "Save data:    " (`KismetStringLibrary.Conv_RotatorToString` (`KismetMathLibrary.InverseTransformRotation` (`SceneComponent.K2_GetComponentToWorld` (`/Game/ThirdPerson/Blueprints/BP_ThirdPersonCharacter.FollowCamera` _asbp_third_person_character)) (`SceneComponent.K2_GetComponentRotation` _lightcomponent_2))) "   Internsity:  " (`KismetStringLibrary.Conv_DoubleToString` (`LightComponentBase.Intensity` _lightcomponent_2)) "   Color: " (`KismetStringLibrary.Conv_ColorToString` (`LightComponentBase.GetLightColor` _lightcomponent_2)) "    Temp:   " (`KismetStringLibrary.Conv_DoubleToString` (`LightComponent.Temperature` _lightcomponent_2)) "    Name: Pic_" (`KismetStringLibrary.Conv_IntToString` (`self.num`)) ".png") true true (struct :`R` 1.0 :`G` 0.08517 :`B` 0.204911 :`A` 1.0) 3.0))))
  (:`Released`
    (set `self.num` (+ (`self.num`) 1))))

(fn `Counter`
  (params (CountNum :type Integer)))

(fn `UserConstructionScript`)