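; Actor that drives a directional light from a JSON file, loading it on BeginPlay and re-reading it every few ticks via a frame counter.
; ReloadJson prints the name field, then applies temperature and intensity to the light.
; It also turns the two "dimention" fields into a vector, rotates it by the player camera's rotation and aims the light along it, making the direction camera-relative.
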(event `Reload Json`
  (bind _directionallight (`self.DirectionalLight`))
  (bind _outjsonobject (`JsonBlueprintFunctionLibrary.FromFile` (`self.json_path`)))
  (`|ExecutionSequence`
    (:`then_0`
      (bind _outvalue (`|GetJsonField` _outjsonobject "name"))
      (`KismetSystemLibrary.PrintString` _outvalue true true (struct :`G` 1.0 :`B` 0.238632 :`A` 1.0) 1.0))
    (:`then_1`
      (bind _outvalue_2 (`|GetJsonField` _outjsonobject "dimention0")))
    (:`then_2`
      (bind _outvalue_3 (`|GetJsonField` _outjsonobject "dimention1")))
    (:`then_3`
      (bind _outvalue_4 (`|GetJsonField` _outjsonobject "temperature"))
      (`LightComponent.SetUseTemperature` _directionallight true)
      (`LightComponent.SetTemperature` _directionallight _outvalue_4))
    (:`then_4`
      (bind _outvalue_5 (`|GetJsonField` _outjsonobject "intensity"))
      (`LightComponent.SetIntensity` _directionallight _outvalue_5))
    (:`then_5`
      (`SceneComponent.K2_SetWorldRotation` _directionallight (`KismetMathLibrary.Conv_VectorToRotator` (`KismetMathLibrary.GreaterGreater_VectorRotator` (`KismetMathLibrary.MakeVector` _outvalue_2 _outvalue_3) (`PlayerCameraManager.GetCameraRotation` (`GameplayStatics.GetPlayerCameraManager` 0)))) false false))))

(event `self.ReceiveBeginPlay`
  (`self.Reload Json`))

(event `self.ReceiveTick`
  (params (DeltaSeconds :type "Float (single-precision)"))
  (if (== (`self.cnt`) 10)
    (set `self.cnt` 0)
    (`self.Reload Json`)
    (else
      (set `self.cnt` (+ (`self.cnt`) 1)))))

(fn `UserConstructionScript`)